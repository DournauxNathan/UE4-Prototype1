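; Enemy hazard that patrols between two points and kills the player on touch.
; On BeginPlay, a latent MoveComponentTo loop shuttles the StaticMesh between EndPos and StartPos over MoveTime, flipping the target after each move.
; StartPos is captured from the actor's world location, yet both targets are applied as relative locations.
; Actor overlap casts to BP_Player and calls Die.
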(event EventBeginPlay
  (Variables|Default|SetstartPos (Transformation|GetActorLocation))
  (Variables|Default|SettargetPos (Variables|Default|GetendPos))
  (Components|MoveComponentTo (Variables|Default|GetStaticMesh) (Variables|Default|GettargetPos) "0, 0, 0" false false (Variables|Default|GetmoveTime) false :!label _label)
  (if (Math|Vector|Equal(Vector) (Variables|Default|GettargetPos) (Variables|Default|GetendPos) 0.0001)
    (Variables|Default|SettargetPos (Variables|Default|GetstartPos))
    (goto _label)
    (else
      (Variables|Default|SettargetPos (Variables|Default|GetendPos))
      (goto _label))))

(event Collision|EventActorBeginOverlap
  (params (OtherActor :type Actor%20Object%20Reference))
  (bind _asbp_player (Utilities|Casting|CastToBP_Player OtherActor))
  (Default|Die _asbp_player))

(fn ConstructionScript)